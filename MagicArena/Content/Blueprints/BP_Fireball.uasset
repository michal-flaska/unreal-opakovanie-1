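; BP_Fireball is a fireball actor that explodes when its sphere component begins overlapping something.
; Overlaps with the player character or with components tagged "sipocka" are ignored.
; Otherwise it spawns a Niagara explosion, runs a small debug-drawn sphere trace in place, prints the overlapped component and traced actor names, then destroys itself.
; The graph applies no damage.
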(event OnComponentBeginOverlap(Sphere)
  (params (OverlappedComponent :type Primitive%20Component%20Object%20Reference) (OtherActor :type Actor%20Object%20Reference) (OtherComp :type Primitive%20Component%20Object%20Reference) (OtherBodyIndex :type Integer) (bFromSweep :type Boolean) (SweepResult :type Hit%20Result%20Structure%20%28by%20ref%29))
  (bind _returnvalue (Transformation|GetActorLocation))
  (if (not (== OtherActor (Game|GetPlayerCharacter 0)))
    (if (not (Components|ComponentHasTag OtherComp "sipocka"))
      (Development|PrintString (Utilities|GetDisplayName OtherComp))
      ;[0.15 0.15 0.15 0.5] Spawn Niagara
      (Niagara|SpawnSystematLocation "/Game/Niagara/NS_FireballExplosion.NS_FireballExplosion" (Transformation|GetActorLocation) (Transformation|GetActorRotation))
      ;[0.15 0.15 0.15 0.5] Tracing
      (bind _outhit (Collision|SphereTraceByChannel _returnvalue _returnvalue 2e+01 "TraceTypeQuery1" false 0 "ForDuration"))
      (Development|PrintString (Utilities|GetDisplayName (.hitactor _outhit)))
      (Actor|DestroyActor))))

(fn ConstructionScript)